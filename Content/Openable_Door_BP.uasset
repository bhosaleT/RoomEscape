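; Openable door actor that swings open and closed when its OpenDoorRightAngle component fires open and close events.
; The DoorSwings timeline plays forward or in reverse, applying its angle as yaw combined with the rotation saved at BeginPlay.
; A timeline event track toggles DoorState to alternate between squeak and lock sounds at the door's location.
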(event `self.ReceiveBeginPlay`
  (set `self.InitialRotation` (`self.K2_GetActorRotation`)))

(event `self.OpenDoorRightAngle.OnOpen`
  (bind _returnvalue (`self.K2_GetActorLocation`))
  (bind (_direction _openangle) (`Timeline|DoorSwings` :!label _label)
    (:`Update`
      (`self.K2_SetActorRotation` (`KismetMathLibrary.ComposeRotators` (`KismetMathLibrary.MakeRotator` 0.0 0.0 _openangle) (`self.InitialRotation`))))
    (:`SoundTiming`
      (if (`self.DoorState`)
        (`GameplayStatics.PlaySoundAtLocation` "/Game/Audio/squeak.squeak" _returnvalue (struct) 1.0 1.0 0.0 null null null)
        (set `self.DoorState` false)
        (else
          (`GameplayStatics.PlaySoundAtLocation` "/Game/Audio/door-lock.door-lock" _returnvalue (struct) 1.0 1.0 0.0 null null null)
          (set `self.DoorState` true))))))

(event `self.OpenDoorRightAngle.OnClose`
  (goto _label :!via `Reverse`))

(fn `UserConstructionScript`)